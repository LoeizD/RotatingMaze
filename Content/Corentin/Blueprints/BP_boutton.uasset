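; BP_boutton is a rotation puzzle button that, when its box is overlapped, turns BP_rot_puzzle_base around X or Y.
; Its world up vector, matched to ±X or ±Y within a tolerance, picks the axis and direction.
; A match disables every button through CanUse and plays a rotation sound, while a DoOnce reset on end overlap prevents repeat triggers.
; Saveposition calls SavePlayer on the base; the cannot-rotate sound is unwired.
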(event OnComponentBeginOverlap(Box)
  (params (OtherActor :type Actor%20Object%20Reference) (OtherComp :type Primitive%20Component%20Object%20Reference) (OtherBodyIndex :type Integer) (bFromSweep :type Boolean) (SweepResult :type Hit%20Result%20Structure%20%28by%20ref%29))
  (bind _angle_tolerance (Variables|Default|Getangle_tolerance))
  (bind _defaultsceneroot (Variables|Default|GetDefaultSceneRoot))
  (bind _returnvalue (Transformation|GetWorldRotation _defaultsceneroot))
  (bind _returnvalue_2 (Math|Vector|GetUpVector _returnvalue))
  (if (Variables|Default|Getcan_use?)
    (Utilities|FlowControl|DoOnce false
      (:Completed
        (Development|PrintString (Utilities|String|ToString(Vector) _returnvalue_2))
        (if (Math|Vector|Equal(Vector) _returnvalue_2 "1.000000,0.000000,0.000000" _angle_tolerance)
          ;[1 1 1] Disable buttons
          (bind _outactors (Actor|GetAllActorsOfClass "BP_boutton_C"))
          (CallFunction|CanUse _outactors false)
          (bind _outactors_2 (Actor|GetAllActorsOfClass "/Game/Corentin/Blueprints/BP_rot_puzzle_base.BP_rot_puzzle_base_C"))
          (Default|RotateY _outactors_2 false)
          (Audio|PlaySound2D "/Game/Corentin/Sounds/rotation_sound.rotation_sound" :!label _label)
          (elif (Math|Vector|Equal(Vector) _returnvalue_2 "-1.000000,0.000000, 0" _angle_tolerance)
            (bind _outactors_3 (Actor|GetAllActorsOfClass "BP_boutton_C"))
            (CallFunction|CanUse _outactors_3 false)
            (bind _outactors_4 (Actor|GetAllActorsOfClass "/Game/Corentin/Blueprints/BP_rot_puzzle_base.BP_rot_puzzle_base_C"))
            (Default|RotateY _outactors_4 true)
            (goto _label)
            (elif (Math|Vector|Equal(Vector) _returnvalue_2 "0.000000,1.000000, 0" _angle_tolerance)
              (bind _outactors_5 (Actor|GetAllActorsOfClass "BP_boutton_C"))
              (CallFunction|CanUse _outactors_5 false)
              (bind _outactors_6 (Actor|GetAllActorsOfClass "/Game/Corentin/Blueprints/BP_rot_puzzle_base.BP_rot_puzzle_base_C"))
              (Default|RotateX _outactors_6 true)
              (goto _label)
              (elif (Math|Vector|Equal(Vector) _returnvalue_2 "0.000000,-1.000000, 0" _angle_tolerance)
                (bind _outactors_7 (Actor|GetAllActorsOfClass "BP_boutton_C"))
                (CallFunction|CanUse _outactors_7 false)
                (bind _outactors_8 (Actor|GetAllActorsOfClass "/Game/Corentin/Blueprints/BP_rot_puzzle_base.BP_rot_puzzle_base_C"))
                (Default|RotateX _outactors_8 false)
                (goto _label)))))))))

(event OnComponentEndOverlap(Box)
  (params (OtherActor :type Actor%20Object%20Reference) (OtherComp :type Primitive%20Component%20Object%20Reference) (OtherBodyIndex :type Integer))
  (bind _angle_tolerance (Variables|Default|Getangle_tolerance))
  (bind _defaultsceneroot (Variables|Default|GetDefaultSceneRoot))
  (bind _returnvalue (Transformation|GetWorldRotation _defaultsceneroot))
  (bind _returnvalue_2 (Math|Vector|GetUpVector _returnvalue))
  (Utilities|FlowControl|DoOnce false) ; enters at Reset
)

(event Custom|Save%20position
  (bind _outactors (Actor|GetAllActorsOfClass "/Game/Corentin/Blueprints/BP_rot_puzzle_base.BP_rot_puzzle_base_C"))
  (Default|SavePlayer _outactors))

(event Custom|can_use
  (params (canUse? :type Boolean))
  (Variables|Default|Setcan_use? canUse?))

(event EventBeginPlay)

(event Collision|EventActorBeginOverlap
  (params (OtherActor :type Actor%20Object%20Reference)))

(event EventTick
  (params (DeltaSeconds :type Float%20%28single-precision%29)))

(fn ConstructionScript)