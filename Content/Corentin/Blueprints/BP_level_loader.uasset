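; Level loader actor that switches maps when its Box component begins an overlap, with no check on which actor entered.
; The overlap opens the level set in LevelToLoad, while a Reset event reopens the one set in CurrentLevel.
; Both derive the level name from an enum's string, and each is gated by its own DoOnce to prevent repeat loads.
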(event OnComponentBeginOverlap(Box)
  (params (OtherActor :type Actor%20Object%20Reference) (OtherComp :type Primitive%20Component%20Object%20Reference) (OtherBodyIndex :type Integer) (bFromSweep :type Boolean) (SweepResult :type Hit%20Result%20Structure%20%28by%20ref%29))
  (Utilities|FlowControl|DoOnce false
    (:Completed
      (Game|OpenLevel(byName) (Utilities|String|StringToName (Utilities|String|EnumtoString (Variables|Default|Getlevel_to_load)))))))

(event Custom|Reset
  (Utilities|FlowControl|DoOnce false
    (:Completed
      (Game|OpenLevel(byName) (Utilities|String|StringToName (Utilities|String|EnumtoString (Variables|Default|Getcurrent_level)))))))

(event EventBeginPlay)

(event Collision|EventActorBeginOverlap
  (params (OtherActor :type Actor%20Object%20Reference)))

(event EventTick
  (params (DeltaSeconds :type Float%20%28single-precision%29)))

(fn ConstructionScript)