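; Base Blueprint for a rotation puzzle that turns its Scene component in quarter turns.
; RotateX and RotateY ease the roll or pitch 90 degrees in either direction over two seconds, then re-enable every BP_boutton in the level.
; A save event stores the player's transform and the Scene's world transform, while the Respawn event is an empty stub.
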(event Custom|RotateY
  (params (negative :type Boolean))
  (bind _scene (Variables|Default|GetScene))
  (bind _relativerotation (Variables|/Script/Engine.SceneComponent|GetRelativeRotation _scene))
  (if negative
    (Components|MoveComponentTo (Variables|Default|GetScene) "0, 0, 0" (Math|Rotator|MakeRotator (+ (.pitch _relativerotation) -9e+01) (.yaw _relativerotation) (.roll _relativerotation)) true true 2.0)
    (else
      (Components|MoveComponentTo (Variables|Default|GetScene) "0, 0, 0" (Math|Rotator|MakeRotator (+ (.pitch _relativerotation) 9e+01) (.yaw _relativerotation) (.roll _relativerotation)) true true 2.0)))
  (bind _outactors (Actor|GetAllActorsOfClass "/Game/Corentin/Blueprints/BP_boutton.BP_boutton_C"))
  (Default|CanUse _outactors true))

(event Custom|save_player
  (Variables|respawn|Setplayer_transform (Transformation|GetActorTransform (Game|GetPlayerCharacter 0)))
  (Variables|Default|Setlevel_transform (Transformation|GetWorldTransform (Variables|Default|GetScene))))

(event Custom|Respawn)

(event Custom|RotateX
  (params (negative? :type Boolean))
  (bind _scene (Variables|Default|GetScene))
  (bind _scene_2 (Variables|Default|GetScene))
  (bind _relativerotation (Variables|/Script/Engine.SceneComponent|GetRelativeRotation _scene_2))
  (if negative?
    (Components|MoveComponentTo _scene "0, 0, 0" (Math|Rotator|MakeRotator 0.0 (.yaw _relativerotation) (+ (.roll _relativerotation) -9e+01)) true true 2.0)
    (else
      (Components|MoveComponentTo _scene "0, 0, 0" (Math|Rotator|MakeRotator (.pitch _relativerotation) (.yaw _relativerotation) (+ (.roll _relativerotation) 9e+01)) true true 2.0)))
  (bind _outactors (Actor|GetAllActorsOfClass "/Game/Corentin/Blueprints/BP_boutton.BP_boutton_C"))
  (Default|CanUse _outactors true))

(fn ConstructionScript)